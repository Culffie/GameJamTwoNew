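; Enemy hover vehicle AI that is meant to ride a track spline, started on BeginPlay when ActiveVehicle is set.
; MoveVehicle plays the VehicleMover timeline from a start offset, with play rate scaled inversely by Duration.
; Each update sets location and rotation from TrackRef's spline, but the distance Lerp's alpha is fixed at zero, pinning the vehicle to the spline start.
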(event `self.ReceiveBeginPlay`
  (if (`self.ActiveVehicle`)
    (`self.MoveVehicle`)))

(event `MoveVehicle`
  (bind _returnvalue (`KismetMathLibrary.Lerp` 0.0 (`SplineComponent.GetSplineLength` (`/Game/HoverVehicle/Track.UsefulSpline` (`self.TrackRef`)))))
  (`TimelineComponent.SetPlayRate` (`self.VehicleMover`) (/ 0.1 (`self.Duration`)))
  (`TimelineComponent.SetNewTime` (`self.VehicleMover`) (`self.VehicleStartOffset`))
  (bind (_direction _alpha) (`Timeline|VehicleMover`)
    (:`Update`
      (set `self.Alpha` _alpha)
      (`self.K2_SetActorLocationAndRotation` (`SplineComponent.GetLocationAtDistanceAlongSpline` (`/Game/HoverVehicle/Track.UsefulSpline` (`self.TrackRef`)) _returnvalue "World") (`SplineComponent.GetRotationAtDistanceAlongSpline` (`/Game/HoverVehicle/Track.UsefulSpline` (`self.TrackRef`)) _returnvalue "World")))))

(fn `UserConstructionScript`)